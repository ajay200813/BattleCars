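; Car pawn Blueprint for BattleCars that manages swapping the guns mounted on a vehicle.
; ReplaceGun sends special weapons to the last array slot and rotates other pickups through the first three slots via a wrapping counter.
; It destroys the old gun, spawns the new class without collision, snaps it to the slot's named socket and updates the Weapons array.
; Event graph and construction script are empty stubs.
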(event EventBeginPlay)

(event EventActorBeginOverlap
  (params (OtherActor :type Actor%20Object%20Reference)))

(event EventTick
  (params (DeltaSeconds :type Float%20%28single-precision%29)))

(fn ConstructionScript)

(fn ReplaceGun
  (params (special :type Boolean :default false) (new_gun :type Actor%20Class%20Reference))
  ;[1 1 1] get which gun slot to replace
  (if special
    (LocalVariables|Setgun_slot (- (Utilities|Array|Length (Variables|Weaponry|Getweapons)) 1))
    (else
      (LocalVariables|Setgun_slot (Variables|Weaponry|Getnext_gun_replaced))
      (CallFunction|SetNextGuntoReplace)))
  ;[1 1 1] destroy gun thats getting replaced
  (Actor|DestroyActor (Utilities|Array|Get(acopy) (Variables|Weaponry|Getweapons) (LocalVariables|Getgun_slot)))
  ;[1 1 1] spawn new gun
  (bind _returnvalue (Game|SpawnActorfromClass new_gun (Math|Transform|MakeTransform "0, 0, 0") true 0))
  (Collision|SetActorEnableCollision _returnvalue false)
  (Class|Actor|AttachRootComponenttoActor _returnvalue self (Utilities|Select :Index (LocalVariables|Getgun_slot) :Option%200 "primary_gun_slot" :Option%201 "secondary_gun_slot" :Option%202 "tertiary_gun_slot" :Option%203 "special_gun_slot") "SnapToTarget" true)
  (Utilities|Casting|CastTovehicle_weapon _returnvalue)
  (Utilities|Array|SetArrayElem (Variables|Weaponry|Getweapons) (LocalVariables|Getgun_slot) 0 true))

(fn SetNextGuntoReplace
  (bind _output_get (Variables|Weaponry|Setnext_gun_replaced (+ (Variables|Weaponry|Getnext_gun_replaced) 1)))
  (if (>= _output_get 3)
    (Variables|Weaponry|Setnext_gun_replaced 0)))