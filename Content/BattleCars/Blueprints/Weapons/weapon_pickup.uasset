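; Base weapon pickup actor for the BattleCars game that gives a gun to a vehicle driving into it.
; On sphere overlap with a base_vehicle, it adds GunType through the vehicle's AddGun, passes the result to WeaponSpecificInit, then destroys itself.
; WeaponSpecificInit is an empty hook returning true, and the Hovering timeline meant to offset the pickup from its start position never runs.
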(event `self.ReceiveBeginPlay`
  (set `self.start_pos` (`self.K2_GetActorLocation`)))

(event `self.ReceiveActorBeginOverlap`
  (params (OtherActor :type "Actor Object Reference")))

(event `self.ReceiveTick`
  (params (DeltaSeconds :type "Float (single-precision)")))

(event `self.Sphere.OnComponentBeginOverlap`
  (params (OtherActor :type "Actor Object Reference") (OtherComp :type "PrimitiveComponent Object Reference") (OtherBodyIndex :type Integer) (bFromSweep :type Boolean) (SweepResult :type "EngineTypes.HitResult Structure (by ref)"))
  (bind _asbase_vehicle (cast `/Game/BattleCars/Blueprints/vehicles/base/base_vehicle` OtherActor))
  ;[1 1 1] add weapon
  (bind _gun (`/Game/BattleCars/Blueprints/vehicles/base/base_vehicle.AddGun` _asbase_vehicle (`self.gun_type`)))
  (`self.weaponSpecificInit` _gun _asbase_vehicle)
  ;[1 1 1] destroy pickup
  (`self.K2_DestroyActor`))

(fn `UserConstructionScript`)

(fn `weaponSpecificInit`
  (params (weapon :type "/Game/BattleCars/Blueprints/Weapons/vehicle_weapon Object Reference") (vehicle :type "/Game/BattleCars/Blueprints/vehicles/base/base_vehicle Object Reference"))
  (returns (success :type Boolean))
  (return true))